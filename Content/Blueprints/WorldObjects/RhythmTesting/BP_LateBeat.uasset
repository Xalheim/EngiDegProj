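; BP_LateBeat is a rhythm-testing actor that visualizes the late-beat window by swapping the material on its cube.
; On BeginPlay it subscribes to sixteenth-note quantization events from the MainRhythmTimer's Quartz clock handle.
; Each event sets orange stripes when the beat fraction falls in a short window just after the beat, and blue geometry otherwise.
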(event Custom|DetectLateBeat
  (params (ClockName :type Name) (QuantizationType :type EQuartzCommandQuantization%20Enum :default "Bar") (NumBars :type Integer) (Beat :type Integer) (BeatFraction :type Float%20%28single-precision%29))
  (bind _cube (Variables|Default|GetCube))
  (if (> BeatFraction 0.1)
    (if (<= BeatFraction 0.3)
      (Rendering|Material|SetMaterial _cube 0 "/Game/Materials/Xals/Test/M_OrangeStripes.M_OrangeStripes")
      (else
        (Rendering|Material|SetMaterial _cube 0 "/Game/Materials/Xals/Test/M_BlueGeometry.M_BlueGeometry" :!label _label)))
    (else
      (goto _label))))

(event EventBeginPlay
  (Class|QuartzClockHandle|SubscribetoQuantizationEvent (Variables|/Game/Blueprints/Gamemodes/BP_MainRhythmTimer.BP_MainRhythmTimer_C|GetClock%20Handle (Variables|Default|GetMainRhythmTimer)) "SixteenthNote" (delegate Custom|DetectLateBeat)))

(event Collision|EventActorBeginOverlap
  (params (OtherActor :type Actor%20Object%20Reference)))

(event EventTick
  (params (DeltaSeconds :type Float%20%28single-precision%29)))

(fn ConstructionScript)