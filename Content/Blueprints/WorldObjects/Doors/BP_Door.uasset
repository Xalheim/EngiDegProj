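; Sliding door actor that opens when the player pawn enters its trigger box and closes when it leaves, unless locked.
; BeginPlay caches closed and open positions from the root location and an offset.
; Tick eases the cube toward either position with VInterpTo, based on the open and locked flags.
; LockDoor and UnlockDoor events set the lock and swap the cube's material, with locking also closing the door.
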(event OnComponentBeginOverlap(Box)
  (params (OverlappedComponent :type Primitive%20Component%20Object%20Reference) (OtherActor :type Actor%20Object%20Reference) (OtherComp :type Primitive%20Component%20Object%20Reference) (OtherBodyIndex :type Integer) (bFromSweep :type Boolean) (SweepResult :type Hit%20Result%20Structure%20%28by%20ref%29))
  (if (== OtherActor (Game|Player|GetPlayerPawn 0))
    (if (not (Variables|Default|GetIsLocked))
      (Variables|Default|SetIsOpen true))))

(event OnComponentEndOverlap(Box)
  (params (OverlappedComponent :type Primitive%20Component%20Object%20Reference) (OtherActor :type Actor%20Object%20Reference) (OtherComp :type Primitive%20Component%20Object%20Reference) (OtherBodyIndex :type Integer))
  (if (== OtherActor (Game|Player|GetPlayerPawn 0))
    (Variables|Default|SetIsOpen false)))

(event Custom|LockDoor
  ;[0.03529 0.03529 0.03529] Lock and Unlock Door from use by Player
  (Variables|Default|SetIsLocked true)
  (Variables|Default|SetIsOpen false)
  (Rendering|Material|SetMaterial (Variables|Default|GetCube) 0 (Variables|Default|GetLockedMaterial)))

(event Custom|UnlockDoor
  ;[0.03529 0.03529 0.03529] Lock and Unlock Door from use by Player
  (Variables|Default|SetIsLocked false)
  (Rendering|Material|SetMaterial (Variables|Default|GetCube) 0 (Variables|Default|GetUnlockedMaterial)))

(event Custom|SetDoorPositions
  (bind _defaultsceneroot (Variables|Default|GetDefaultSceneRoot))
  (bind _returnvalue (Transformation|GetWorldLocation _defaultsceneroot))
  ;[0.03529 0.03529 0.03529] Set vectors for opened and closed door
  (Variables|Default|SetDoorClosePosition _returnvalue)
  (Variables|Default|SetDoorOpenPosition (+ _returnvalue (Variables|Default|GetDoorOpenDistance))))

(event EventBeginPlay
  (CallFunction|SetDoorPositions))

(event EventTick
  (params (DeltaSeconds :type Float%20%28single-precision%29))
  (if (Variables|Default|GetIsOpen)
    (if (Variables|Default|GetIsLocked)
      (Transformation|SetWorldLocation (Variables|Default|GetCube) (Math|Interpolation|VInterpTo (Transformation|GetWorldLocation (Variables|Default|GetCube)) (Variables|Default|GetDoorClosePosition) DeltaSeconds 4.0) false false :!label _label)
      (else
        (Transformation|SetWorldLocation (Variables|Default|GetCube) (Math|Interpolation|VInterpTo (Transformation|GetWorldLocation (Variables|Default|GetCube)) (Variables|Default|GetDoorOpenPosition) DeltaSeconds 4.0) false false)))
    (else
      (goto _label))))

(fn ConstructionScript)