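; BP_MainRhythmTimer runs the game's rhythm clock and tracks timing accuracy, rhythm score and score multiplier.
; On BeginPlay it creates a Quartz clock at the set BPM, playing a sound at the player pawn on each beat.
; Sixteenth-note events grade the current accuracy window from the beat fraction.
; ModifyRhythmScore clamps the running score and derives a tiered 1x to 4x multiplier from it.
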(event Custom|CheckMultiplier
  (bind _rhythmscore (Variables|Default|GetRhythmScore))
  (if (>= _rhythmscore 4.8e+02)
    (Variables|Default|SetRhythmMultiplier 4)
    (elif (>= _rhythmscore 1.8e+02)
      (Variables|Default|SetRhythmMultiplier 3)
      (elif (>= _rhythmscore 6e+01)
        (Variables|Default|SetRhythmMultiplier 2)
        (else
          (Variables|Default|SetRhythmMultiplier 1))))))

(event Custom|Start%20Rhythm%20Timer
  (if (> (Variables|Default|GetBPM) 0.0)
    (Variables|Default|SetIsRhythmClockRunning true)
    ;[0.03529 0.03529 0.03529] Create Quartz Clock for rhythm timing
    (bind _returnvalue (Class|QuartzSubsystem|CreateNewClock (WorldSubsystems|GetQuartzSubsystem) (Variables|Default|GetClock%20Name) (Utilities|Struct|MakeQuartzClockSettings (Utilities|Struct|MakeQuartzTimeSignature 4 "QuarterNote") false) false))
    (bind _output_get (Variables|Default|SetClock%20Handle _returnvalue))
    (bind _clockhandle (Class|QuartzClockHandle|SetBeatsPerMinute _output_get (Utilities|Struct|MakeQuartzQuantizationBoundary "Bar" 4.0 "BarRelative") 0 (Variables|Default|GetBPM)))
    (bind _clockhandle_2 (Class|QuartzClockHandle|StartClock _clockhandle))
    (Class|QuartzClockHandle|SubscribetoQuantizationEvent _clockhandle_2 "Beat" (delegate Custom|beatsound))
    (Class|QuartzClockHandle|SubscribetoQuantizationEvent (Variables|Default|GetClock%20Handle) "SixteenthNote" (delegate Custom|Set%20Rhythm%20Accuracy))
    (else
      ;[0.03529 0.03529 0.03529] Invalid BPM should block any action or return to menu
      (Development|PrintString "NO BPM SET, SHOULD RETURN TO MENU/ RAISE ERROR/ DISALLOW RUN OF MAP" true true "(R=1.000000,G=0.000000,B=0.000000,A=1.000000)" 2e+01))))

(event Custom|ModifyRhythmScore
  (params (B :type Float%20%28double-precision%29))
  (Variables|Default|SetRhythmScore (Math|Float|Clamp(Float) (+ (Variables|Default|GetRhythmScore) B) 0.0 5.2e+02))
  (CallFunction|CheckMultiplier))

(event Custom|Stop%20Rhythm%20Timer
  (if (Variables|Default|GetIsRhythmClockRunning)
    (Variables|Default|SetIsRhythmClockRunning false)))

(event Custom|beatsound
  (params (ClockName :type Name) (QuantizationType :type EQuartzCommandQuantization%20Enum :default "Bar") (NumBars :type Integer) (Beat :type Integer) (BeatFraction :type Float%20%28single-precision%29))
  (Audio|PlaySoundatLocation "/Game/Sounds/Player_Throw.Player_Throw" (Transformation|GetActorLocation (Game|Player|GetPlayerPawn 0)) "0, 0, 0" 0.3 1.0 0.0 0 0 0 0))

(event Custom|Set%20Rhythm%20Accuracy
  (params (ClockName :type Name) (QuantizationType :type EQuartzCommandQuantization%20Enum :default "Bar") (NumBars :type Integer) (Beat :type Integer) (BeatFraction :type Float%20%28single-precision%29))
  (if (>= BeatFraction 0.5)
    (if (>= BeatFraction 0.9)
      (Variables|Default|SetCurrentRhythmAccuracy "NewEnumerator0")
      (elif (>= BeatFraction 0.7)
        (Variables|Default|SetCurrentRhythmAccuracy "NewEnumerator2")
        (else
          (Variables|Default|SetCurrentRhythmAccuracy "NewEnumerator3"))))
    (elif (<= BeatFraction 0.1)
      (Variables|Default|SetCurrentRhythmAccuracy "NewEnumerator0")
      (elif (<= BeatFraction 0.3)
        (Variables|Default|SetCurrentRhythmAccuracy "NewEnumerator1")
        (else
          (Variables|Default|SetCurrentRhythmAccuracy "NewEnumerator3"))))))

(event EventBeginPlay
  (CallFunction|StartRhythmTimer))

(fn ConstructionScript)