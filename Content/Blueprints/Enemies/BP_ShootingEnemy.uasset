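; Ranged enemy that chases the player and fires projectiles in time with the music.
; Pawn sensing turns it toward the player, then either follows with AI MoveTo when far or stops to attack when in range.
; A Quartz beat subscription drives attacks: a random beat countdown, an aim cue on one beat, then an impulse-launched projectile and short recovery.
; Tick swaps single-node animations whenever the selected state changes.
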(event OnSeePawn(PawnSensing)
  (params (Pawn :type Pawn%20Object%20Reference))
  (Transformation|SetActorRotation (Math|Conversions|RotationFromXVector (Math|Vector|Normalize (- (Transformation|GetActorLocation (Game|Player|GetPlayerPawn 0)) (Transformation|GetWorldLocation (Variables|Default|GetCapsuleComponent))))))
  (if (not (Variables|Default|GetIsAttacking))
    (if (> (Math|Vector|Distance(Vector) (Transformation|GetActorLocation (Game|Player|GetPlayerPawn 0)) (Transformation|GetActorLocation)) 2e+03)
      (CallFunction|FollowPlayer)
      (elif (not (Variables|Default|GetIsRecovering))
        (CallFunction|AttackPlayer)))))

(event Custom|Follow%20Player
  (Variables|Default|SetSelectedAnimation "NewEnumerator1")
  (AI|AIMoveTo self "0, 0, 0" (Game|Player|GetPlayerPawn 0) 5.0 false))

(event Custom|Attack%20Player
  (Variables|Default|SetSelectedAnimation "NewEnumerator2")
  (Class|NavMovementComponent|StopActiveMovement (Variables|Character|GetCharacterMovement))
  (Variables|Default|SetIsAttacking true))

(event Custom|Try%20Attack
  (params (ClockName :type Name) (QuantizationType :type EQuartzCommandQuantization%20Enum :default "Bar") (NumBars :type Integer) (Beat :type Integer) (BeatFraction :type Float%20%28single-precision%29))
  (if (Variables|Default|GetIsAttacking)
    (if (> (Variables|Default|GetShotDelay) 0)
      (Variables|Default|SetShotDelay (- (Variables|Default|GetShotDelay) 1))
      (elif (Variables|Default|GetIsAiming)
        (CallFunction|ShootPlayer)
        (Audio|PlaySoundatLocation "/Game/FPWeapon/Audio/FirstPersonTemplateWeaponFire02.FirstPersonTemplateWeaponFire02" (Transformation|GetWorldLocation (Variables|Default|GetCapsuleComponent)) "0, 0, 0" 0.5 1.0 0.0 0 0 0 0)
        (else
          (Variables|Default|SetIsAiming true)
          (Audio|PlaySoundatLocation "/Game/Sounds/Mov_Dash.Mov_Dash" (Transformation|GetWorldLocation (Variables|Default|GetCapsuleComponent)) "0, 0, 0" 0.3 1.0 0.0 0 0 0 0)
          (Variables|Default|SetSelectedAnimation "NewEnumerator2"))))))

(event Custom|Shoot%20Player
  (bind _returnvalue (Transformation|GetActorTransform))
  (bind _self self)
  (Variables|Default|SetSelectedAnimation "NewEnumerator3")
  (Variables|Default|SetIsAttacking false)
  (Variables|Default|SetIsAiming false)
  (Variables|Default|SetIsRecovering true)
  (Variables|Default|SetShotDelay (+ (Math|Random|RandomInteger 6) 2))
  (bind _returnvalue_2 (Game|SpawnActorfromClass "/Game/Blueprints/Projectiles/BasicProjectile.BasicProjectile_C" (Math|Transform|MakeTransform (+ (.location _returnvalue) "0.000000,0.000000,35.000000") (.rotation _returnvalue) (.scale _returnvalue)) "AlwaysSpawn" "OverrideRootScale" _self _self))
  (Physics|AddImpulse (Variables|/Game/Blueprints/Projectiles/BasicProjectile.BasicProjectile_C|GetCylinder _returnvalue_2) (* (Variables|/Game/Blueprints/Projectiles/BP_ParentProjectile.BP_ParentProjectile_C|GetTravelSpeed _returnvalue_2) (Math|Vector|Normalize (- (Transformation|GetActorLocation (Game|Player|GetPlayerPawn 0)) (Transformation|GetWorldLocation (Variables|/Game/Blueprints/Projectiles/BasicProjectile.BasicProjectile_C|GetCylinder _returnvalue_2))))) "None" false)
  (Transformation|SetActorRotation _returnvalue_2 (Math|Conversions|RotationFromXVector (Math|Vector|Normalize (- (Transformation|GetActorLocation (Game|Player|GetPlayerPawn 0)) (Transformation|GetWorldLocation (Variables|/Game/Blueprints/Projectiles/BasicProjectile.BasicProjectile_C|GetCylinder _returnvalue_2))))))
  (Utilities|FlowControl|Delay 1.0)
  (Variables|Default|SetIsRecovering false))

(event EventBeginPlay
  (|CallParentFunction)
  (Class|QuartzClockHandle|SubscribetoQuantizationEvent (Variables|/Game/Blueprints/Gamemodes/BP_MainRhythmTimer.BP_MainRhythmTimer_C|GetClock%20Handle (Variables|Default|GetMainRhythmTimer)) "Beat" (delegate Custom|Try%20Attack))
  (Components|Animation|OverrideAnimationData (Variables|Character|GetMesh) "/Game/Models/ShootingEnemy/ED_ShootingEnemy_Anim_ArmatureBones_Idle.ED_ShootingEnemy_Anim_ArmatureBones_Idle" true true 0.0 1.0)
  (Variables|Default|SetShotDelay (Math|Random|RandomInteger 4)))

(event Collision|EventActorBeginOverlap
  (params (OtherActor :type Actor%20Object%20Reference))
  (|CallParentFunction 0))

(event EventTick
  (params (DeltaSeconds :type Float%20%28single-precision%29))
  (bind _mesh (Variables|Character|GetMesh))
  (|CallParentFunction DeltaSeconds)
  (if (not (Utilities|Enum|Equal(Enum) (Variables|Default|GetSelectedAnimation) (Variables|Default|GetCurrentAnimation)))
    (Variables|Default|SetCurrentAnimation (Variables|Default|GetSelectedAnimation))
    (switch Utilities|FlowControl|Switch|SwitchonShootingEnemyStates (Variables|Default|GetCurrentAnimation)
      (:NewEnumerator0
        (Components|Animation|PlayAnimation _mesh "/Game/Models/ShootingEnemy/ED_ShootingEnemy_Anim_ArmatureBones_Idle.ED_ShootingEnemy_Anim_ArmatureBones_Idle" true))
      (:NewEnumerator1
        (Components|Animation|PlayAnimation _mesh "/Game/Models/ShootingEnemy/ED_ShootingEnemy_Anim_ArmatureBones_Walk.ED_ShootingEnemy_Anim_ArmatureBones_Walk" true))
      (:NewEnumerator2
        (Components|Animation|PlayAnimation _mesh "/Game/Models/ShootingEnemy/ED_ShootingEnemy_Anim_ArmatureBones_Aim.ED_ShootingEnemy_Anim_ArmatureBones_Aim" true))
      (:NewEnumerator3
        (Components|Animation|PlayAnimation _mesh "/Game/Models/ShootingEnemy/ED_ShootingEnemy_Anim_ArmatureBones_Shoot.ED_ShootingEnemy_Anim_ArmatureBones_Shoot" false)))))

(fn ConstructionScript
  (|CallParentFunction))