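; Pillar is a rhythm-driven boss for a VR player, with three spinning cubes, contact damage and a health bar on the player.
; Quartz clock events from BP_MainRhythmTimer fire four radial projectiles each beat and, from phase two, opposed laser walls each bar.
; While active, Tick rotates the cubes and checks health, dropping barriers at phase thresholds and enabling damaging main lasers in phase three.
; Death resets the pillar, then loads the main menu after a delay.
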(event OnComponentHit(BoxDamageCollision)
  (params (HitComponent :type Primitive%20Component%20Object%20Reference) (OtherActor :type Actor%20Object%20Reference) (OtherComp :type Primitive%20Component%20Object%20Reference) (NormalImpulse :type Vector :default "0, 0, 0") (Hit :type Hit%20Result%20Structure%20%28by%20ref%29))
  (bind _returnvalue (Game|Player|GetPlayerPawn 0))
  (if (== OtherActor _returnvalue)
    (if (not (Variables|Default|GetCloseHit))
      (Variables|Default|SetCloseHit true)
      (Game|Damage|ApplyDamage _returnvalue 5e+01 0 0)
      (Utilities|FlowControl|Delay 0.3)
      (Variables|Default|SetCloseHit false))))

(event OnComponentBeginOverlap(LaserOne)
  (params (OverlappedComponent :type Primitive%20Component%20Object%20Reference) (OtherActor :type Actor%20Object%20Reference) (OtherComp :type Primitive%20Component%20Object%20Reference) (OtherBodyIndex :type Integer) (bFromSweep :type Boolean) (SweepResult :type Hit%20Result%20Structure%20%28by%20ref%29))
  (bind _returnvalue (Game|Player|GetPlayerPawn 0))
  (if (Variables|Default|GetThirdPhase)
    (if (== OtherActor _returnvalue)
      (Game|Damage|ApplyDamage _returnvalue 2e+01 0 0))))

(event OnComponentBeginOverlap(LaserTwo)
  (params (OverlappedComponent :type Primitive%20Component%20Object%20Reference) (OtherActor :type Actor%20Object%20Reference) (OtherComp :type Primitive%20Component%20Object%20Reference) (OtherBodyIndex :type Integer) (bFromSweep :type Boolean) (SweepResult :type Hit%20Result%20Structure%20%28by%20ref%29))
  (bind _returnvalue (Game|Player|GetPlayerPawn 0))
  (if (Variables|Default|GetThirdPhase)
    (if (== OtherActor _returnvalue)
      (Game|Damage|ApplyDamage _returnvalue 2e+01 0 0))))

(event Custom|ShootBullet
  (params (ClockName :type Name) (QuantizationType :type EQuartzCommandQuantization%20Enum :default "Bar") (NumBars :type Integer) (Beat :type Integer) (BeatFraction :type Float%20%28single-precision%29))
  (if (Variables|Default|GetActive)
    (if (not (Variables|Default|GetDead))
      (CallFunction|ShootGun1))))

(event Custom|Check%20Health
  (bind _health (Variables|Default|GetHealth))
  (Rendering|Components|TextRender|SetText (Variables|/Game/Blueprints/Player/VRPawn.VRPawn_C|GetBossHealthBarNumber (Variables|Default|GetPlayer)) (Utilities|Text|ToText(Float) (Variables|Default|GetHealth) "HalfToEven"))
  (if (<= _health 0.0)
    (CallFunction|ResetPillar)
    (Variables|Default|SetDead true)
    (Rendering|SetVisibility (Variables|/Game/Blueprints/Player/VRPawn.VRPawn_C|GetBossHealthBarNumber (Variables|Default|GetPlayer)) true false)
    (Utilities|FlowControl|Delay 4.0)
    (Game|OpenLevel(byObjectReference) "/Game/Levels/MainMenu.MainMenu")
    (elif (<= _health 1e+03)
      (if (not (Variables|Default|GetThirdPhase))
        (Variables|Default|SetThirdPhase true)
        (Rendering|SetVisibility (Variables|Default|GetLaserBarrier3) false false)
        (for _array_element (Components|GetChildrenComponents (Variables|Default|GetMainLaser) false)
          (Rendering|SetVisibility _array_element true false)))
      (elif (<= _health 2.5e+03)
        (if (not (Variables|Default|GetSecondPhase))
          (Variables|Default|SetSecondPhase true)
          (Rendering|SetVisibility (Variables|Default|GetLaserBarrier2) false false))))))

(event Custom|Reset%20Pillar
  (Variables|Default|SetDead false)
  (Variables|Default|SetActive false)
  (Variables|Default|SetHealth 4e+03)
  (Variables|Default|SetSecondPhase false)
  (Variables|Default|SetThirdPhase false)
  (Rendering|SetVisibility (Variables|/Game/Blueprints/Player/VRPawn.VRPawn_C|GetBossHealthBarNumber (Variables|Default|GetPlayer)) false false)
  (for _array_element (Components|GetChildrenComponents (Variables|Default|GetMainLaser) false)
    (Rendering|SetVisibility _array_element false false))
  (Rendering|SetVisibility (Variables|Default|GetLaserBarrier3) true false)
  (Rendering|SetVisibility (Variables|Default|GetLaserBarrier2) true false)
  (Variables|/Game/Blueprints/Gamemodes/BP_MainRhythmTimer.BP_MainRhythmTimer_C|SetIsPlayerFighting (Variables|Default|GetMainRhythmTimer) false))

(event Custom|FireLaserWalls
  (params (ClockName :type Name) (QuantizationType :type EQuartzCommandQuantization%20Enum :default "Bar") (NumBars :type Integer) (Beat :type Integer) (BeatFraction :type Float%20%28single-precision%29))
  (if (Variables|Default|GetActive)
    (if (not (Variables|Default|GetDead))
      (if (Variables|Default|GetSecondPhase)
        (CallFunction|ShootLaserWall)))))

(event Custom|ActivatePillar
  (Variables|Default|SetActive true)
  (Rendering|SetVisibility (Variables|/Game/Blueprints/Player/VRPawn.VRPawn_C|GetBossHealthBarNumber (Variables|Default|GetPlayer)) true false)
  (Variables|/Game/Blueprints/Gamemodes/BP_MainRhythmTimer.BP_MainRhythmTimer_C|SetIsPlayerFighting (Variables|Default|GetMainRhythmTimer) true))

(event Custom|ShootGun1
  (bind _cube1 (Variables|Default|GetCube1))
  (bind _cube1_2 (Variables|Default|GetCube1))
  (bind _cube1_gun1 (Variables|Default|GetCube1_Gun1))
  (bind _cube1_gun1_2 (Variables|Default|GetCube1_Gun1))
  (bind _cube1_3 (Variables|Default|GetCube1))
  (bind _cube1_gun2 (Variables|Default|GetCube1_Gun2))
  (bind _cube1_gun2_2 (Variables|Default|GetCube1_Gun2))
  (bind _cube1_4 (Variables|Default|GetCube1))
  (bind _cube1_gun3 (Variables|Default|GetCube1_Gun3))
  (bind _cube1_gun3_2 (Variables|Default|GetCube1_Gun3))
  (bind _cube1_gun4 (Variables|Default|GetCube1_Gun4))
  (bind _cube1_gun4_2 (Variables|Default|GetCube1_Gun4))
  (bind _returnvalue (Transformation|GetWorldTransform _cube1_gun1))
  (bind _returnvalue_2 (Transformation|GetWorldLocation _cube1_2))
  (bind _returnvalue_3 (Transformation|GetWorldLocation _cube1_gun1_2))
  (bind _returnvalue_4 (Transformation|GetWorldTransform _cube1_gun2_2))
  (bind _returnvalue_5 (Transformation|GetWorldLocation _cube1_4))
  (bind _returnvalue_6 (Transformation|GetWorldLocation _cube1_gun2))
  (bind _returnvalue_7 (Transformation|GetWorldTransform _cube1_gun3))
  (bind _returnvalue_8 (Transformation|GetWorldLocation _cube1_3))
  (bind _returnvalue_9 (Transformation|GetWorldLocation _cube1_gun3_2))
  (bind _returnvalue_10 (Transformation|GetWorldLocation _cube1))
  (bind _returnvalue_11 (Transformation|GetWorldLocation _cube1_gun4))
  (bind _returnvalue_12 (Transformation|GetWorldTransform _cube1_gun4_2))
  (bind _returnvalue_13 (- _returnvalue_11 _returnvalue_10))
  (bind _returnvalue_14 (- _returnvalue_3 _returnvalue_2))
  (bind _returnvalue_15 (- _returnvalue_6 _returnvalue_5))
  (bind _returnvalue_16 (- _returnvalue_9 _returnvalue_8))
  (bind _returnvalue_17 (Game|SpawnActorfromClass "/Game/Blueprints/Projectiles/BasicProjectile.BasicProjectile_C" (Math|Transform|MakeTransform (.location _returnvalue) (Math|Rotator|CombineRotators (.rotation _returnvalue) "0.000000,90.000000,0.000000") "1.000000,1.000000,1.000000") "Undefined" "MultiplyWithRoot" 0 0))
  (Physics|AddImpulse (Variables|/Game/Blueprints/Projectiles/BasicProjectile.BasicProjectile_C|GetCylinder _returnvalue_17) (* (Math|Vector|Normalize (Math|Vector|MakeVector (.x _returnvalue_14) (.y _returnvalue_14) 0.0)) (Variables|/Game/Blueprints/Projectiles/BP_ParentProjectile.BP_ParentProjectile_C|GetTravelSpeed _returnvalue_17)) "None" false)
  (bind _returnvalue_18 (Game|SpawnActorfromClass "/Game/Blueprints/Projectiles/BasicProjectile.BasicProjectile_C" (Math|Transform|MakeTransform (.location _returnvalue_4) (Math|Rotator|CombineRotators (.rotation _returnvalue_4) "0.000000,90.000000,0.000000") "1.000000,1.000000,1.000000") "Undefined" "MultiplyWithRoot" 0 0))
  (Physics|AddImpulse (Variables|/Game/Blueprints/Projectiles/BasicProjectile.BasicProjectile_C|GetCylinder _returnvalue_18) (* (Math|Vector|Normalize (Math|Vector|MakeVector (.x _returnvalue_15) (.y _returnvalue_15) 0.0)) (Variables|/Game/Blueprints/Projectiles/BP_ParentProjectile.BP_ParentProjectile_C|GetTravelSpeed _returnvalue_18)) "None" false)
  (bind _returnvalue_19 (Game|SpawnActorfromClass "/Game/Blueprints/Projectiles/BasicProjectile.BasicProjectile_C" (Math|Transform|MakeTransform (.location _returnvalue_7) (Math|Rotator|CombineRotators (.rotation _returnvalue_7) "0.000000,90.000000,0.000000") "1.000000,1.000000,1.000000") "Undefined" "MultiplyWithRoot" 0 0))
  (Physics|AddImpulse (Variables|/Game/Blueprints/Projectiles/BasicProjectile.BasicProjectile_C|GetCylinder _returnvalue_19) (* (Math|Vector|Normalize (Math|Vector|MakeVector (.x _returnvalue_16) (.y _returnvalue_16) 0.0)) (Variables|/Game/Blueprints/Projectiles/BP_ParentProjectile.BP_ParentProjectile_C|GetTravelSpeed _returnvalue_19)) "None" false)
  (bind _returnvalue_20 (Game|SpawnActorfromClass "/Game/Blueprints/Projectiles/BasicProjectile.BasicProjectile_C" (Math|Transform|MakeTransform (.location _returnvalue_12) (Math|Rotator|CombineRotators (.rotation _returnvalue_12) "0.000000,90.000000,0.000000") "1.000000,1.000000,1.000000") "Undefined" "MultiplyWithRoot" 0 0))
  (Physics|AddImpulse (Variables|/Game/Blueprints/Projectiles/BasicProjectile.BasicProjectile_C|GetCylinder _returnvalue_20) (* (Math|Vector|Normalize (Math|Vector|MakeVector (.x _returnvalue_13) (.y _returnvalue_13) 0.0)) (Variables|/Game/Blueprints/Projectiles/BP_ParentProjectile.BP_ParentProjectile_C|GetTravelSpeed _returnvalue_20)) "None" false))

(event Custom|ShootLaserWall
  (bind _cube2 (Variables|Default|GetCube2))
  (bind _returnvalue (Math|Vector|GetForwardVector _cube2))
  (bind _returnvalue_2 (Math|Vector|Normalize _returnvalue))
  (bind _returnvalue_3 (* _returnvalue_2 "4000.000000,4000.000000,0.000000"))
  (bind _returnvalue_4 (Game|SpawnActorfromClass "/Game/Blueprints/Projectiles/Lasers/DashableLaserWall.DashableLaserWall_C" (Math|Transform|MakeTransform (+ (Transformation|GetSocketLocation (Variables|Default|GetDefaultSceneRoot) "None") "0.000000,0.000000,300.000000") (Transformation|GetWorldRotation (Variables|Default|GetCube2)) "1.000000,5.000000,1.000000") "Undefined" "MultiplyWithRoot" 0 0))
  (Physics|AddImpulse (Variables|/Game/Blueprints/Projectiles/Lasers/DashableLaserWall.DashableLaserWall_C|GetCube _returnvalue_4) _returnvalue_3 "None" false)
  (bind _returnvalue_5 (Game|SpawnActorfromClass "/Game/Blueprints/Projectiles/Lasers/DashableLaserWall.DashableLaserWall_C" (Math|Transform|MakeTransform (+ (Transformation|GetSocketLocation (Variables|Default|GetDefaultSceneRoot) "None") "0.000000,0.000000,300.000000") (Transformation|GetWorldRotation (Variables|Default|GetCube2)) "1.000000,5.000000,1.000000") "Undefined" "MultiplyWithRoot" 0 0))
  (Physics|AddImpulse (Variables|/Game/Blueprints/Projectiles/Lasers/DashableLaserWall.DashableLaserWall_C|GetCube _returnvalue_5) (Math|Vector|NegateVector _returnvalue_3) "None" false))

(event EventBeginPlay
  (for _array_element (Components|GetChildrenComponents (Variables|Default|GetMainLaser) false)
    (Rendering|SetVisibility _array_element false false))
  (bind _outactors (Actor|GetAllActorsOfClass "/Game/Blueprints/Gamemodes/BP_MainRhythmTimer.BP_MainRhythmTimer_C"))
  (bind _output_get (Variables|Default|SetMainRhythmTimer (Utilities|Array|Get(acopy) _outactors)))
  (bind _clockhandle (Class|QuartzClockHandle|SubscribetoQuantizationEvent (Variables|/Game/Blueprints/Gamemodes/BP_MainRhythmTimer.BP_MainRhythmTimer_C|GetClock%20Handle _output_get) "Beat" (delegate Custom|ShootBullet)))
  (Class|QuartzClockHandle|SubscribetoQuantizationEvent _clockhandle "Bar" (delegate Custom|FireLaserWalls))
  (Utilities|FlowControl|DelayUntilNextTick)
  (bind _asvrpawn (Utilities|Casting|CastToVRPawn (Game|Player|GetPlayerPawn 0)))
  (Variables|Default|SetPlayer _asvrpawn))

(event Collision|EventActorBeginOverlap
  (params (OtherActor :type Actor%20Object%20Reference)))

(event Game|Damage|EventAnyDamage
  (params (Damage :type Float%20%28single-precision%29) (DamageType :type Damage%20Type%20Object%20Reference) (InstigatedBy :type Controller%20Object%20Reference) (DamageCauser :type Actor%20Object%20Reference))
  (Variables|Default|SetHealth (- (Variables|Default|GetHealth) Damage)))

(event EventTick
  (params (DeltaSeconds :type Float%20%28single-precision%29))
  (bind _cube1 (Variables|Default|GetCube1))
  (bind _cube2 (Variables|Default|GetCube2))
  (bind _cube3 (Variables|Default|GetCube3))
  (bind _returnvalue (Transformation|GetWorldRotation _cube3))
  (bind _returnvalue_2 (Transformation|GetWorldRotation _cube1))
  (bind _returnvalue_3 (Transformation|GetWorldRotation _cube2))
  (if (Variables|Default|GetActive)
    (Variables|Default|SetDelta DeltaSeconds)
    (CallFunction|CheckHealth)
    (Transformation|SetWorldRotation (Variables|Default|GetCube1) (Class|KismetMathLibrary|RInterptoConstant _returnvalue_2 (Math|Rotator|CombineRotators _returnvalue_2 "0.000000,60.000000,0.000000") (Variables|Default|GetDelta) 2e+01) false false)
    (Transformation|SetWorldRotation (Variables|Default|GetCube2) (Class|KismetMathLibrary|RInterptoConstant _returnvalue_3 (Math|Rotator|CombineRotators _returnvalue_3 "0.000000,-60.000000,0.000000") (Variables|Default|GetDelta) 1e+01) false false)
    (Transformation|SetWorldRotation (Variables|Default|GetCube3) (Class|KismetMathLibrary|RInterptoConstant _returnvalue (Math|Rotator|CombineRotators _returnvalue "0.000000,60.000000,0.000000") (Variables|Default|GetDelta) 6e+01) false false)))

(fn ConstructionScript)