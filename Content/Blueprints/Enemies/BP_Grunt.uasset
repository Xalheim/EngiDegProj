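; BP_Grunt is an enemy that uses PawnSensing to chase or shoot at the player.
; On seeing a pawn, it measures distance to player 0, moving toward them beyond a threshold and otherwise stopping to attack.
; An IsAttacking flag and Delay throttle projectile spawns, with a sound after each delay.
; Projectiles spawn at the grunt-minus-player offset vector, raised in Z, with zero rotation, rather than at the grunt's location.
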(event OnSeePawn(PawnSensing)
  (params (Pawn :type Pawn%20Object%20Reference))
  (if (> (Math|Vector|Distance(Vector) (Transformation|GetActorLocation (Game|Player|GetPlayerPawn 0)) (Transformation|GetActorLocation)) 6e+02)
    (CallFunction|FollowPlayer)
    (else
      (CallFunction|AttackPlayer))))

(event Custom|Follow%20Player
  (AI|AIMoveTo self "0, 0, 0" (Game|Player|GetPlayerPawn 0) 5.0 false))

(event Custom|Attack%20Player
  (bind _self self)
  (Class|NavMovementComponent|StopActiveMovement (Variables|Character|GetCharacterMovement))
  (if (not (Variables|Default|GetIsAttacking))
    (Variables|Default|SetIsAttacking true)
    (Game|SpawnActorfromClass "/Game/Blueprints/Projectiles/Projectile.Projectile_C" (Math|Transform|MakeTransform (+ (- (.location (Transformation|GetActorTransform)) (Transformation|GetActorLocation (Game|Player|GetPlayerPawn 0))) "0.000000,0.000000,100.000000")) "AlwaysSpawn" "OverrideRootScale" _self _self)
    (Utilities|FlowControl|Delay 0.5)
    (Variables|Default|SetIsAttacking false)
    (Audio|PlaySound2D "/Game/Sounds/RhPs_NoAmmo.RhPs_NoAmmo" 1.0 1.0 0.0 0 0)))

(event EventBeginPlay
  (|CallParentFunction))

(event Collision|EventActorBeginOverlap
  (params (OtherActor :type Actor%20Object%20Reference))
  (|CallParentFunction 0))

(event EventTick
  (params (DeltaSeconds :type Float%20%28single-precision%29))
  (|CallParentFunction DeltaSeconds) ; This node is disabled and will not be called.\nDrag off pins to build functionality.
)

(fn ConstructionScript
  (|CallParentFunction))