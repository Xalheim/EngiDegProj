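; Melee enemy that chases the player and swings in time with the music.
; PawnSensing turns it toward the player, moving it with AIMoveTo or starting an attack when close.
; A Quartz beat subscription winds up on one beat and strikes the next, damaging a player in range, then applies beat-counted cooldown and timed recovery.
; Tick plays mesh animations directly whenever the selected state changes, without an AnimBP state machine.
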(event OnSeePawn(PawnSensing)
  (params (Pawn :type Pawn%20Object%20Reference))
  (Transformation|SetActorRotation (Math|Conversions|RotationFromXVector (Math|Vector|Normalize (- (Transformation|GetActorLocation (Game|Player|GetPlayerPawn 0)) (Transformation|GetWorldLocation (Variables|Default|GetCapsuleComponent))))))
  (if (not (Variables|Default|GetIsAttacking))
    (if (> (Math|Vector|Distance(Vector) (Transformation|GetActorLocation (Game|Player|GetPlayerPawn 0)) (Transformation|GetActorLocation)) 3e+02)
      (CallFunction|FollowPlayer)
      (elif (not (Variables|Default|GetIsRecovering))
        (CallFunction|AttackPlayer)))))

(event Custom|Try%20Swing
  (params (ClockName :type Name) (QuantizationType :type EQuartzCommandQuantization%20Enum :default "Bar") (NumBars :type Integer) (Beat :type Integer) (BeatFraction :type Float%20%28single-precision%29))
  (Utilities|FlowControl|Sequence
    (:then_0
      (if (> (Variables|Default|GetShotDelay) 0)
        (Variables|Default|SetShotDelay (- (Variables|Default|GetShotDelay) 1))))
    (:then_1
      (if (Variables|Default|GetIsAttacking)
        (if (not (> (Variables|Default|GetShotDelay) 0))
          (if (Variables|Default|GetIsAiming)
            (CallFunction|MeleePlayer)
            (Audio|PlaySoundatLocation "/Game/Sounds/Mov_Dash.Mov_Dash" (Transformation|GetWorldLocation (Variables|Default|GetCapsuleComponent)) "0, 0, 0" 0.5 0.4 0.0 0 0 0 0)
            (else
              (Variables|Default|SetIsAiming true)
              (Audio|PlaySoundatLocation "/Game/Sounds/RhPs_Reload.RhPs_Reload" (Transformation|GetWorldLocation (Variables|Default|GetCapsuleComponent)) "0, 0, 0" 0.3 0.4 0.0 0 0 0 0)
              (Variables|Default|SetSelectedAnimation "NewEnumerator2"))))))))

(event Custom|Melee%20Player
  (bind _returnvalue (Game|Player|GetPlayerPawn 0))
  (Class|NavMovementComponent|StopActiveMovement (Variables|Character|GetCharacterMovement))
  (Variables|Default|SetSelectedAnimation "NewEnumerator3")
  (if (< (Math|Vector|Distance(Vector) (Transformation|GetActorLocation (Game|Player|GetPlayerPawn 0)) (Transformation|GetWorldLocation (Variables|Character|GetMesh))) 2.5e+02)
    (Game|Damage|ApplyDamage _returnvalue 25.0 0 0))
  (Variables|Default|SetIsAttacking false)
  (bind _asvrpawn (Utilities|Casting|CastToVRPawn _returnvalue))
  (Development|PrintString (Utilities|String|ToString(Float) (Variables|/Game/Blueprints/Player/VRPawn.VRPawn_C|GetHealth _asvrpawn)))
  (Variables|Default|SetIsAiming false)
  (Variables|Default|SetIsRecovering true)
  (Variables|Default|SetShotDelay 4)
  (Utilities|FlowControl|Delay 1.0)
  (Variables|Default|SetIsRecovering false))

(event Custom|Attack%20Player
  (Variables|Default|SetSelectedAnimation "NewEnumerator2")
  (Variables|Default|SetIsAttacking true))

(event Custom|Follow%20Player
  (Variables|Default|SetSelectedAnimation "NewEnumerator1")
  (AI|AIMoveTo self "0, 0, 0" (Game|Player|GetPlayerPawn 0) 5.0 false))

(event EventBeginPlay
  (|CallParentFunction)
  (Class|QuartzClockHandle|SubscribetoQuantizationEvent (Variables|/Game/Blueprints/Gamemodes/BP_MainRhythmTimer.BP_MainRhythmTimer_C|GetClock%20Handle (Variables|Default|GetMainRhythmTimer)) "Beat" (delegate Custom|Try%20Swing))
  (Components|Animation|OverrideAnimationData (Variables|Character|GetMesh) "/Game/Models/ShootingEnemy/ED_ShootingEnemy_Anim_ArmatureBones_Idle.ED_ShootingEnemy_Anim_ArmatureBones_Idle" true true 0.0 1.0))

(event Collision|EventActorBeginOverlap
  (params (OtherActor :type Actor%20Object%20Reference))
  (|CallParentFunction OtherActor))

(event EventTick
  (params (DeltaSeconds :type Float%20%28single-precision%29))
  (bind _mesh (Variables|Character|GetMesh))
  (|CallParentFunction DeltaSeconds)
  (if (not (Utilities|Enum|Equal(Enum) (Variables|Default|GetSelectedAnimation) (Variables|Default|GetCurrentAnimation)))
    (Variables|Default|SetCurrentAnimation (Variables|Default|GetSelectedAnimation))
    (switch Utilities|FlowControl|Switch|SwitchonMeleeEnemyStates (Variables|Default|GetCurrentAnimation)
      (:NewEnumerator0
        (Components|Animation|PlayAnimation _mesh "/Game/Models/MeleeEnemy/ED_MeleeEnemy_Anim_ArmatureBones_Idle.ED_MeleeEnemy_Anim_ArmatureBones_Idle" true))
      (:NewEnumerator1
        (Components|Animation|PlayAnimation _mesh "/Game/Models/MeleeEnemy/ED_MeleeEnemy_Anim_ArmatureBones_Walk.ED_MeleeEnemy_Anim_ArmatureBones_Walk" true))
      (:NewEnumerator2
        (Components|Animation|PlayAnimation _mesh "/Game/Models/MeleeEnemy/ED_MeleeEnemy_Anim_ArmatureBones_Aim.ED_MeleeEnemy_Anim_ArmatureBones_Aim" true))
      (:NewEnumerator3
        (Components|Animation|PlayAnimation _mesh "/Game/Models/MeleeEnemy/ED_MeleeEnemy_Anim_ArmatureBones_Swing.ED_MeleeEnemy_Anim_ArmatureBones_Swing" false)))))

(fn ConstructionScript
  (|CallParentFunction))