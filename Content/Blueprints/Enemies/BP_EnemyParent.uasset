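; BP_EnemyParent is a base enemy Blueprint that gives enemies health and death handling.
; AnyDamage subtracts incoming damage from Health.
; Tick polls Health every frame and, once it reaches zero or below, plays a death sound at the capsule's location and destroys the actor.
; BeginPlay and the construction script are empty.
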(event EventBeginPlay)

(event EventTick
  (params (DeltaSeconds :type Float%20%28single-precision%29))
  ;[0.03529 0.03529 0.03529] Check if enemy ran out of health
  (if (<= (Variables|Default|GetHealth) 0.0)
    (Audio|PlaySoundatLocation "/Game/Sounds/EnemySFX_Death1_EnemySFX_Death1.EnemySFX_Death1_EnemySFX_Death1" (Transformation|GetWorldLocation (Variables|Collision|GetCapsuleComponent)) "0, 0, 0" 1.0 1.0 0.0 0 0 0 0)
    (Actor|DestroyActor)))

(event Game|Damage|EventAnyDamage
  (params (Damage :type Float%20%28single-precision%29) (DamageType :type Damage%20Type%20Object%20Reference) (InstigatedBy :type Controller%20Object%20Reference) (DamageCauser :type Actor%20Object%20Reference))
  ;[0.03529 0.03529 0.03529] Apply damage to enemy
  (Variables|Default|SetHealth (- (Variables|Default|GetHealth) Damage)))

(fn ConstructionScript)