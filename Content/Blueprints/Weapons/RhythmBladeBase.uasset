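; Base grabbable melee blade for rhythm combat that damages enemies and pillars on overlap and scores each hit by timing accuracy.
; A block capsule destroys projectiles to build parry charge, which adds to the next hit's damage, then resets.
; A Quartz bar subscription on the main rhythm timer drains that charge over time.
; Dropping enables physics, letting the capsule serve as an in-flight hitbox until the blade destroys itself on impact or timeout.
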(event OnComponentBeginOverlap(RhythmBlade)
  (params (OverlappedComponent :type Primitive%20Component%20Object%20Reference) (OtherActor :type Actor%20Object%20Reference) (OtherComp :type Primitive%20Component%20Object%20Reference) (OtherBodyIndex :type Integer) (bFromSweep :type Boolean) (SweepResult :type Hit%20Result%20Structure%20%28by%20ref%29))
  (bind _returnvalue (Utilities|GetClass OtherActor))
  ;[0.03529 0.03529 0.03529] If Blade collides with enemy, apply damage and Parry Charge, then reset Parry Charge.
  (if (Utilities|ClassIsChildOf _returnvalue "/Game/Blueprints/Enemies/BP_EnemyParent.BP_EnemyParent_C")
    (bind _asbp_enemy_parent (Utilities|Casting|CastToBP_EnemyParent OtherActor))
    (if (not (Variables|/Game/Blueprints/Enemies/BP_EnemyParent.BP_EnemyParent_C|GetIsMeleeHit _asbp_enemy_parent))
      (Default|MeleeDelay _asbp_enemy_parent)
      (CallFunction|ApplyMeleeDamage _asbp_enemy_parent)
      (Audio|PlaySound2D "/Game/Sounds/RhPs_Hitsound.RhPs_Hitsound" 0.4 1.4 0.0 0 0 :!label _label))
    (elif (Utilities|ClassIsChildOf _returnvalue "/Game/Blueprints/Enemies/Pillar.Pillar_C")
      (CallFunction|ApplyMeleeDamage OtherActor)
      (goto _label))))

(event OnComponentHit(RhythmBlade)
  (params (HitComponent :type Primitive%20Component%20Object%20Reference) (OtherActor :type Actor%20Object%20Reference) (OtherComp :type Primitive%20Component%20Object%20Reference) (NormalImpulse :type Vector :default "0, 0, 0") (Hit :type Hit%20Result%20Structure%20%28by%20ref%29))
  (if (not (== OtherActor (Game|Player|GetPlayerPawn 0)))
    (Actor|DestroyActor)))

(event OnComponentBeginOverlap(CapsuleBlock)
  (params (OverlappedComponent :type Primitive%20Component%20Object%20Reference) (OtherActor :type Actor%20Object%20Reference) (OtherComp :type Primitive%20Component%20Object%20Reference) (OtherBodyIndex :type Integer) (bFromSweep :type Boolean) (SweepResult :type Hit%20Result%20Structure%20%28by%20ref%29))
  ;[0.03529 0.03529 0.03529] If Block Capsule collides with projectile, destroy the projectile and add Parry Charge up to 250.
  (if (Utilities|ClassIsChildOf (Utilities|GetClass OtherActor) "/Game/Blueprints/Projectiles/BasicProjectile.BasicProjectile_C")
    (Actor|DestroyActor OtherActor)
    (if (>= (Variables|Default|GetParryCharge) 200)
      _
      (else
        (Variables|Default|SetParryCharge (+ (Variables|Default|GetParryCharge) 30))))
    (Audio|PlaySound2D "/Game/Sounds/RhPs_Reload.RhPs_Reload" 0.6 1.2 0.0 0 0)
    (elif (== (Utilities|GetClass OtherActor) "/Game/Blueprints/WorldObjects/Tutorial/BreakableMelee_Blueprint.BreakableMelee_Blueprint_C")
      (Actor|DestroyActor)
      (else
        ;[0.03529 0.03529 0.03529] If weapon is flying, use bigger hitbox to hit objects easier mid flight.
        (if (Physics|IsSimulatingPhysics (Variables|Default|GetRhythmBlade) "None")
          (if (not (== OtherActor (Game|Player|GetPlayerPawn 0)))
            (bind _asbp_enemy_parent (Utilities|Casting|CastToBP_EnemyParent OtherActor)
              (:then
                (CallFunction|ApplyMeleeDamage _asbp_enemy_parent))
              (:CastFailed
                (Actor|DestroyActor)))))))))

(event OnComponentHit(CapsuleBlock)
  (params (HitComponent :type Primitive%20Component%20Object%20Reference) (OtherActor :type Actor%20Object%20Reference) (OtherComp :type Primitive%20Component%20Object%20Reference) (NormalImpulse :type Vector :default "0, 0, 0") (Hit :type Hit%20Result%20Structure%20%28by%20ref%29))
  (Development|PrintString "CAPSULE BLOCK COMPONENT HIT")
  (Development|PrintString (Utilities|GetDisplayName OtherActor))
  (if (== (Utilities|GetClass OtherActor) "/Game/Blueprints/WorldObjects/Tutorial/BreakableMelee_Blueprint.BreakableMelee_Blueprint_C")
    (Actor|DestroyActor OtherActor)))

(event OnGrabbed(GrabComponent)
  ;[0.03434 0.03434 0.03434] When the Blade is grabbed, disable physics. Re-enable upon drop.
  (Physics|SetSimulatePhysics (Variables|Default|GetRhythmBlade) false))

(event OnDropped(GrabComponent)
  ;[0.03434 0.03434 0.03434] When the Blade is grabbed, disable physics. Re-enable upon drop.
  (Physics|SetSimulatePhysics (Variables|Default|GetRhythmBlade) true)
  (Utilities|FlowControl|Delay 4.0)
  (Actor|DestroyActor))

(event Custom|Lower%20Parry%20Damage
  (params (ClockName :type Name) (QuantizationType :type EQuartzCommandQuantization%20Enum :default "Bar") (NumBars :type Integer) (Beat :type Integer) (BeatFraction :type Float%20%28single-precision%29))
  (Utilities|FlowControl|DelayUntilNextTick)
  (if (> (Variables|Default|GetParryCharge) 0)
    (Variables|Default|SetParryCharge (- (Variables|Default|GetParryCharge) 5))))

(event Custom|ApplyMeleeDamage
  (params (Enemy :type Actor%20Object%20Reference))
  (bind _mainrhythmtimer (Variables|Default|GetMainRhythmTimer))
  (Game|Damage|ApplyDamage Enemy (+ (Variables|Default|GetParryCharge) (Variables|Default|GetMeleeDamage)) (Game|GetPlayerController 0) (Game|Player|GetPlayerPawn 0))
  (Variables|Default|SetParryCharge 0)
  ;[0.03529 0.03529 0.03529] Modify score based on timing accuracy
  (switch Utilities|FlowControl|Switch|SwitchonAccuracyTypes (Variables|/Game/Blueprints/Gamemodes/BP_MainRhythmTimer.BP_MainRhythmTimer_C|GetCurrentRhythmAccuracy (Variables|Default|GetMainRhythmTimer))
    (:NewEnumerator0
      (Default|ModifyRhythmScore _mainrhythmtimer 15.0)
      (Development|PrintString "Perfect"))
    (:NewEnumerator1
      (Default|ModifyRhythmScore _mainrhythmtimer 1e+01)
      (Development|PrintString "Early"))
    (:NewEnumerator2
      (Default|ModifyRhythmScore _mainrhythmtimer 1e+01)
      (Development|PrintString "Late"))
    (:NewEnumerator3
      (Default|ModifyRhythmScore _mainrhythmtimer -15.0)
      (Development|PrintString "Missed"))))

(event Custom|EnableParryDropoff
  (Class|QuartzClockHandle|SubscribetoQuantizationEvent (Variables|/Game/Blueprints/Gamemodes/BP_MainRhythmTimer.BP_MainRhythmTimer_C|GetClock%20Handle (Variables|Default|GetMainRhythmTimer)) "Bar" (delegate Custom|Lower%20Parry%20Damage)))

(event EventBeginPlay
  (bind _outactors (Actor|GetAllActorsOfClass "/Game/Blueprints/Gamemodes/BP_MainRhythmTimer.BP_MainRhythmTimer_C"))
  (Variables|Default|SetMainRhythmTimer (Utilities|Array|Get(acopy) _outactors))
  (CallFunction|EnableParryDropoff))

(event EventTick
  (params (DeltaSeconds :type Float%20%28single-precision%29)))

(fn ConstructionScript)