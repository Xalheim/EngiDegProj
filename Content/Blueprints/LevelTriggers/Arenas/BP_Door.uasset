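; BP_Door is a lockable door in the arena level triggers that opens while overlapped and closes when an overlap ends.
; BeginPlay caches the closed position and an open position offset by DoorOpenDistance, and Tick snaps the root to one based on IsOpen, without interpolation.
; LockDoor forces it shut and blocks overlap opening until UnlockDoor is called.
; Overlaps are not filtered by actor type.
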(event Custom|LockDoor
  ;[0.03529 0.03529 0.03529] Lock and Unlock Door from use by Player
  (Variables|Default|SetIsLocked true)
  (Variables|Default|SetIsOpen false))

(event Custom|UnlockDoor
  ;[0.03529 0.03529 0.03529] Lock and Unlock Door from use by Player
  (Variables|Default|SetIsLocked false))

(event Custom|SetDoorPositions
  (bind _defaultsceneroot (Variables|Default|GetDefaultSceneRoot))
  (bind _returnvalue (Transformation|GetWorldLocation _defaultsceneroot))
  ;[0.03529 0.03529 0.03529] Set vectors for opened and closed door
  (Variables|Default|SetDoorClosePosition _returnvalue)
  (Variables|Default|SetDoorOpenPosition (+ _returnvalue (Variables|Default|GetDoorOpenDistance))))

(event EventBeginPlay
  (CallFunction|SetDoorPositions))

(event Collision|EventActorBeginOverlap
  (params (OtherActor :type Actor%20Object%20Reference))
  (if (not (Variables|Default|GetIsLocked))
    (Variables|Default|SetIsOpen true)))

(event EventTick
  (params (DeltaSeconds :type Float%20%28single-precision%29))
  (if (Variables|Default|GetIsOpen)
    (Transformation|SetWorldLocation (Variables|Default|GetDefaultSceneRoot) (Variables|Default|GetDoorOpenPosition) false false)
    (else
      (Transformation|SetWorldLocation (Variables|Default|GetDefaultSceneRoot) (Variables|Default|GetDoorClosePosition) false false))))

(event Collision|EventActorEndOverlap
  (params (OtherActor :type Actor%20Object%20Reference))
  (Variables|Default|SetIsOpen false))

(fn ConstructionScript)