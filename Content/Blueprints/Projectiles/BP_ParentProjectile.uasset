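; BP_ParentProjectile is, by its name, the base projectile that damages the player or enemies on contact.
; Overlapping the player pawn, or a BP_EnemyParent descendant other than its owner, applies Damage and destroys the projectile, so enemies can hit one another.
; Other overlaps are ignored, while any Hit event or a four-second lifetime timeout also destroys it, with debug prints for outcomes.
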(event EventBeginPlay
  (Utilities|FlowControl|Delay 4.0)
  (Actor|DestroyActor)
  (Development|PrintString "Time's up, destroyed projectile!"))

(event EventTick
  (params (DeltaSeconds :type Float%20%28single-precision%29)))

(event Collision|EventActorBeginOverlap
  (params (OtherActor :type Actor%20Object%20Reference))
  (bind _returnvalue (Game|Player|GetPlayerPawn 0))
  ;[0.03529 0.03529 0.03529] If projectile hits player, apply damage.    If projectile hits a non-enemy, kill projectile.    If projectile hits other enemy, apply damage to the enemy.
  (if (== OtherActor _returnvalue)
    (Game|Damage|ApplyDamage _returnvalue (Math|Conversions|ToFloat(Integer) (Variables|Default|GetDamage)) 0 0)
    (Actor|DestroyActor)
    (Development|PrintString "Player hit!")
    (elif (Utilities|ClassIsChildOf (Utilities|GetClass OtherActor) "/Game/Blueprints/Enemies/BP_EnemyParent.BP_EnemyParent_C")
      (if (not (== OtherActor (Components|GetOwner)))
        (Game|Damage|ApplyDamage OtherActor (Math|Conversions|ToFloat(Integer) (Variables|Default|GetDamage)) 0 0)
        (Actor|DestroyActor)
        (Development|PrintString "hit enemy")))))

(event Collision|EventHit
  (params (MyComp :type Primitive%20Component%20Object%20Reference) (Other :type Actor%20Object%20Reference) (OtherComp :type Primitive%20Component%20Object%20Reference) (bSelfMoved :type Boolean) (HitLocation :type Vector :default "0, 0, 0") (HitNormal :type Vector :default "0, 0, 0") (NormalImpulse :type Vector :default "0, 0, 0") (Hit :type Hit%20Result%20Structure%20%28by%20ref%29))
  (Actor|DestroyActor)
  (Development|PrintString "Hit something"))

(fn ConstructionScript)